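; Animated double door that swings Door01 and Door02 toward open or closed rotations, opening automatically on BeginPlay.
; Open sets targets from the stored starting world rotations plus per-door offsets, subtracting yaw on the second door, while Close restores the starting rotations.
; Tick eases roll, pitch and yaw separately toward the targets with FInterpTo and applies the results as world rotations.
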(event Custom|Open
  (bind _openrotation_door01 (Variables|Default|GetOpenRotation_Door01))
  (bind _openrotation_door02 (Variables|Default|GetOpenRotation_Door02))
  (bind _startingrotation_door01 (Variables|Default|GetStartingRotation_Door01))
  (bind _startingrotation_door02 (Variables|Default|GetStartingRotation_Door02))
  (Variables|Default|SetTargetRotation_Door01 (Math|Rotator|MakeRotator (+ (.roll _startingrotation_door01) (.roll _openrotation_door01)) (+ (.pitch _startingrotation_door01) (.pitch _openrotation_door01)) (+ (.yaw _startingrotation_door01) (.yaw _openrotation_door01))))
  (Variables|Default|SetTargetRotation_Door02 (Math|Rotator|MakeRotator (+ (.roll _startingrotation_door02) (.roll _openrotation_door02)) (+ (.pitch _startingrotation_door02) (.pitch _openrotation_door02)) (- (.yaw _startingrotation_door02) (.yaw _openrotation_door02)))))

(event Custom|Close
  (Variables|Default|SetTargetRotation_Door01 (Variables|Default|GetStartingRotation_Door01))
  (Variables|Default|SetTargetRotation_Door02 (Variables|Default|GetStartingRotation_Door02)))

(event EventBeginPlay
  (Variables|Default|SetStartingRotation_Door01 (Transformation|GetWorldRotation (Variables|Default|GetDoor01)))
  (Variables|Default|SetStartingRotation_Door02 (Transformation|GetWorldRotation (Variables|Default|GetDoor02)))
  (CallFunction|Open))

(event Collision|EventActorBeginOverlap
  (params (OtherActor :type Actor%20Object%20Reference)))

(event EventTick
  (params (DeltaSeconds :type Float%20%28single-precision%29))
  (bind _targetrotation_door01 (Variables|Default|GetTargetRotation_Door01))
  (bind _targetrotation_door02 (Variables|Default|GetTargetRotation_Door02))
  (Variables|Default|SetCurrentRotation_Door01 (Math|Rotator|MakeRotator (Math|Interpolation|FInterpTo (.roll (Variables|Default|GetCurrentRotation_Door01)) (.roll _targetrotation_door01) DeltaSeconds 6.0) (Math|Interpolation|FInterpTo (.pitch (Variables|Default|GetCurrentRotation_Door01)) (.pitch _targetrotation_door01) DeltaSeconds 6.0) (Math|Interpolation|FInterpTo (.yaw (Variables|Default|GetCurrentRotation_Door01)) (.yaw _targetrotation_door01) DeltaSeconds 6.0)))
  (Variables|Default|SetCurrentRotation_Door02 (Math|Rotator|MakeRotator (Math|Interpolation|FInterpTo (.roll (Variables|Default|GetCurrentRotation_Door02)) (.roll _targetrotation_door02) DeltaSeconds 6.0) (Math|Interpolation|FInterpTo (.pitch (Variables|Default|GetCurrentRotation_Door02)) (.pitch _targetrotation_door02) DeltaSeconds 6.0) (Math|Interpolation|FInterpTo (.yaw (Variables|Default|GetCurrentRotation_Door02)) (.yaw _targetrotation_door02) DeltaSeconds 6.0)))
  (Transformation|SetWorldRotation (Variables|Default|GetDoor01) (Variables|Default|GetCurrentRotation_Door01) false false)
  (Transformation|SetWorldRotation (Variables|Default|GetDoor02) (Variables|Default|GetCurrentRotation_Door02) false false))

(fn ConstructionScript)