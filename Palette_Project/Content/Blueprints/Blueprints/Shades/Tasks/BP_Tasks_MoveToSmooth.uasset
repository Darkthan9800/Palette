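; Behavior tree task for Shade AI that moves the controlled pawn toward the player.
; On execute, it casts the owner to the Shade controller and runs AI MoveTo on the blackboard's player reference with a small acceptance radius.
; It finishes successfully on arrival, while the AI tick fails it if the in-paint blackboard flag is set.
; A failed move has no handler, so it does not finish the task.
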(event EventReceiveExecute
  (params (OwnerActor :type Actor%20Object%20Reference))
  (bind _asbp_shade_controller (Utilities|Casting|CastToBP_Shade_Controller OwnerActor))
  (AI|AIMoveTo (Pawn|GetControlledPawn _asbp_shade_controller) (Pawn|GetControlledPawn _asbp_shade_controller) "0, 0, 0" (AI|BehaviorTree|GetBlackboardValueasActor (Variables|Default|GetBBKeyPlayerRef)) 15.0 false
    (:OnSuccess
      (AI|BehaviorTree|FinishExecute true))))

(event EventReceiveTickAI
  (params (OwnerController :type AI%20Controller%20Object%20Reference) (ControlledPawn :type Pawn%20Object%20Reference) (DeltaSeconds :type Float%20%28single-precision%29))
  (if (Class|BTFunctionLibrary|GetBlackboardValueasBool (Variables|Default|GetBBKeyIsInPaint))
    (AI|BehaviorTree|FinishExecute false)))