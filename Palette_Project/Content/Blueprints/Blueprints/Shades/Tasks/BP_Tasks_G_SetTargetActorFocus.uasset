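; Behavior tree task that points a Shade AI's focus at a viable target it can see.
; On execute, it loops through the controller's sight-perceived actors and compares each exact class with the first three ViableTargets entries on the controlled Shade.
; Each match becomes the focus, so the last one wins, and the task finishes with the IsFocusSet flag as its result.
; A loop break hangs off Tick instead of the loop body.
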(event EventReceiveExecute
  (params (OwnerActor :type Actor%20Object%20Reference))
  (bind _asbp_shade_controller (Utilities|Casting|CastToBP_Shade_Controller OwnerActor))
  (bind _output_get (Variables|Default|SetAs%20BP%20Shade%20Controller _asbp_shade_controller))
  (bind _asbp_shade_base (Utilities|Casting|CastToBP_Shade_Base (Pawn|GetControlledPawn _asbp_shade_controller)))
  (bind _output_get_2 (Variables|Default|SetAs%20BP%20Shade%20Base _asbp_shade_base))
  (bind _array_element (Utilities|Array|ForEachLoopwithBreak (Class|AIPerceptionComponent|GetPerceivedActors (Variables|/Game/Blueprints/Blueprints/Shades/BP_Shade_Controller.BP_Shade_Controller_C|GetAIPerception _output_get) "/Script/AIModule.AISense_Sight"))
    (:LoopBody
      (if (Math|Boolean|ORBoolean (== (Utilities|GetClass _array_element) (Utilities|Array|Get(acopy) (Variables|/Game/Blueprints/Blueprints/Shades/BP_Shade_Base.BP_Shade_Base_C|GetViableTargets _output_get_2))) (== (Utilities|GetClass _array_element) (Utilities|Array|Get(acopy) (Variables|/Game/Blueprints/Blueprints/Shades/BP_Shade_Base.BP_Shade_Base_C|GetViableTargets _output_get_2) 1)) (== (Utilities|GetClass _array_element) (Utilities|Array|Get(acopy) (Variables|/Game/Blueprints/Blueprints/Shades/BP_Shade_Base.BP_Shade_Base_C|GetViableTargets _output_get_2) 2)))
        (AI|SetFocus (Variables|Default|GetAs%20BP%20Shade%20Controller) _array_element)
        (Variables|Default|SetIsFocusSet true)))
    (:Completed
      (AI|BehaviorTree|FinishExecute (Variables|Default|GetIsFocusSet)))))

(event EventTick
  (params (OwnerActor :type Actor%20Object%20Reference) (DeltaSeconds :type Float%20%28single-precision%29))
  (if (Variables|Default|GetIsFocusSet)
    (Utilities|Array|ForEachLoopwithBreak (Class|AIPerceptionComponent|GetPerceivedActors (Variables|/Game/Blueprints/Blueprints/Shades/BP_Shade_Controller.BP_Shade_Controller_C|GetAIPerception (stale EventReceiveExecute _output_get)) "/Script/AIModule.AISense_Sight")) ; enters at Break
  ))