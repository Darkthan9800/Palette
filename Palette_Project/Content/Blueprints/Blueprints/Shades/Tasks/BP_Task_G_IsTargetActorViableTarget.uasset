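; Behavior tree task that checks whether a Shade AI's current target is a viable target type.
; It compares the class of the TargetActor blackboard object against the ViableTargets list on the controlled Shade pawn.
; A match sets Success, which is never reset in the graph, then printed and returned through FinishExecute.
; A failed controller or pawn cast exits without finishing the task.
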(event EventReceiveExecute
  (params (OwnerActor :type Actor%20Object%20Reference))
  (bind _asbp_shade_controller (Utilities|Casting|CastToBP_Shade_Controller OwnerActor))
  (bind _asbp_shade_base (Utilities|Casting|CastToBP_Shade_Base (Pawn|GetControlledPawn _asbp_shade_controller)))
  (bind _output_get (Variables|Default|SetShade _asbp_shade_base))
  (for _array_element (Variables|/Game/Blueprints/Blueprints/Shades/BP_Shade_Base.BP_Shade_Base_C|GetViableTargets _output_get)
    (if (== _array_element (Utilities|GetClass (AI|Components|Blackboard|GetValueasObject (AI|GetBlackboard _asbp_shade_controller) (Utilities|Name|MakeLiteralName "TargetActor"))))
      (Variables|Default|SetSuccess true)))
  (Development|PrintString (Utilities|String|ToString(Boolean) (Variables|Default|GetSuccess)))
  (AI|BehaviorTree|FinishExecute (Variables|Default|GetSuccess)))