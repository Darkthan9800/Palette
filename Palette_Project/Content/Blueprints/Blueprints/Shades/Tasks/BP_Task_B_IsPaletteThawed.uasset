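; BP_Task_B_IsPaletteThawed is a behavior tree task for Shade AI that checks whether the player easel's palette is thawed.
; It casts the player pawn to BP_Pawn_Easel and reads the inverse of its palette's IsFrozen flag.
; The result is written to the IsPaletteThawed blackboard key and also becomes the task's success or failure.
; If the cast fails, the task never calls FinishExecute.
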(event EventReceiveExecute
  (params (OwnerActor :type Actor%20Object%20Reference))
  (bind _asbp_pawn_easel (Utilities|Casting|CastToBP_Pawn_Easel (Game|Player|GetPlayerPawn 0)))
  (Variables|Default|SetAs%20BP%20Pawn%20Easel _asbp_pawn_easel)
  (bind _output_get (Variables|Default|SetIsPaletteThawed (Math|Boolean|NotEqual(Boolean) (Variables|/Game/Blueprints/Blueprints/BP_Pawn_Palette.BP_Pawn_Palette_C|GetIsFrozen (Variables|/Game/Blueprints/Blueprints/BP_Pawn_Easel.BP_Pawn_Easel_C|GetPaletteReference (Variables|Default|GetAs%20BP%20Pawn%20Easel))) true)))
  (AI|Components|Blackboard|SetValueasBool (AI|GetBlackboard (AI|GetAIController 0)) (Utilities|Name|MakeLiteralName "IsPaletteThawed") _output_get)
  (AI|BehaviorTree|FinishExecute _output_get))