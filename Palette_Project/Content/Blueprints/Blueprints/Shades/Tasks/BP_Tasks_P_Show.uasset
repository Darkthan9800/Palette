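; Behavior tree task that makes the Paranoia shade show itself.
; On execute it casts the owner to the shade controller and its controlled pawn to the Paranoia shade, storing both references.
; It then calls Show on the shade, sets the IsHidden blackboard key to false and finishes successfully.
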(event EventReceiveExecute
  (params (OwnerActor :type Actor%20Object%20Reference))
  (Utilities|FlowControl|Sequence
    (:then_0
      (bind _asbp_shade_controller (Utilities|Casting|CastToBP_Shade_Controller OwnerActor))
      (bind _output_get (Variables|Default|SetAs%20BP%20Shade%20Controller _asbp_shade_controller))
      (bind _asbp_shade_paranoia (Utilities|Casting|CastToBP_Shade_Paranoia (Pawn|GetControlledPawn _output_get)))
      (Variables|Default|SetAs%20BP%20Shade%20Paranoia _asbp_shade_paranoia))
    (:then_1
      (Default|Show (Variables|Default|GetAs%20BP%20Shade%20Paranoia))
      (AI|Components|Blackboard|SetValueasBool (AI|GetBlackboard (Variables|Default|GetAs%20BP%20Shade%20Controller)) (Utilities|Name|MakeLiteralName "IsHidden") false)
      (AI|BehaviorTree|FinishExecute true))))