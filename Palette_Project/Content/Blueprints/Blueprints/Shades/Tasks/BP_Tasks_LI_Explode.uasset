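; Behavior tree task that makes a Lingering shade explode and splatter shade paint around itself.
; It calls Explode on the controlled pawn, then spawns a random handful of BP_Shade_PaintObject actors at random navigable points nearby.
; It then destroys overlapping WorldDynamic BP_PaintObject actors within the same radius around the pawn and finishes successfully.
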(event EventReceiveExecute
  (params (OwnerActor :type Actor%20Object%20Reference))
  (bind _asbp_shade_controller (Utilities|Casting|CastToBP_Shade_Controller OwnerActor))
  (bind _output_get (Variables|Default|SetAs%20BP%20Shade%20Controller _asbp_shade_controller))
  (Utilities|FlowControl|Sequence
    (:then_0
      (Development|PrintString "Explode")
      (bind _asbp_shade_lingering (Utilities|Casting|CastToBP_Shade_Lingering (Pawn|GetControlledPawn (Variables|Default|GetAs%20BP%20Shade%20Controller))))
      (Default|Explode _asbp_shade_lingering))
    (:then_1
      (for _index (range 0 (Math|Random|RandomIntegerinRange 5 9))
        (Game|SpawnActorfromClass "/Game/Blueprints/Blueprints/BP_Shade_PaintObject.BP_Shade_PaintObject_C" (Math|Transform|MakeTransform (.RandomLocation (Class|NavigationSystemV1|GetRandomPointinNavigableRadius (Transformation|GetActorLocation (Pawn|GetControlledPawn (Variables|Default|GetAs%20BP%20Shade%20Controller))) 4e+02 0 0))) "AlwaysSpawn" 0 -1 0)))
    (:then_2
      (bind _outactors (Collision|SphereOverlapActors (Transformation|GetActorLocation (Pawn|GetControlledPawn _output_get)) 4e+02 (Utilities|Array|MakeArray "ObjectTypeQuery2") "/Game/Blueprints/Blueprints/BP_PaintObject.BP_PaintObject_C"))
      (for _array_element _outactors
        (Actor|DestroyActor _array_element))
      (AI|BehaviorTree|FinishExecute true))))