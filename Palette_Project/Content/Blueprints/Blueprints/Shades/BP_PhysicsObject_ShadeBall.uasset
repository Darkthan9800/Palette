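; A physics shade ball that moves vertically each tick and bursts into paint shades when overlapped by a fishing pole.
; Tick offsets the sphere's Z from the actor location by rate of motion times direction.
; Overlapping a kill volume destroys it outright.
; A fishing pole overlap triggers, once, several paint shade spawns at random reachable nearby points, an ink explosion effect and sound, then delayed destruction.
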(event OnComponentBeginOverlap(Sphere)
  (params (OverlappedComponent :type Primitive%20Component%20Object%20Reference) (OtherActor :type Actor%20Object%20Reference) (OtherComp :type Primitive%20Component%20Object%20Reference) (OtherBodyIndex :type Integer) (bFromSweep :type Boolean) (SweepResult :type Hit%20Result%20Structure%20%28by%20ref%29))
  (bind _returnvalue (Utilities|GetClass OtherActor))
  (if (== _returnvalue "/Game/Blueprints/Blueprints/BP_KillVolume.BP_KillVolume_C")
    (Actor|DestroyActor)
    (elif (== _returnvalue "/Game/Blueprints/Blueprints/InteractableObjects/BP_InteractableObject_FishingPole.BP_InteractableObject_FishingPole_C")
      (Utilities|FlowControl|DoOnce false
        (:Completed
          (for _index (range 0 (Math|Random|RandomIntegerinRange 5 9))
            (Game|SpawnActorfromClass "/Game/Blueprints/Blueprints/BP_Shade_PaintObject.BP_Shade_PaintObject_C" (Math|Transform|MakeTransform (.RandomLocation (AI|Navigation|GetRandomReachablePointinRadius (Transformation|GetActorLocation) 1.5e+02 0 0))) "AlwaysSpawn" 0 -1 false 0))
          (Components|Activation|Activate (Variables|Default|GetInkExplosion) true)
          (Audio|PlaySoundatLocation "/Game/StarterContent/Audio/Explosion02.Explosion02" (Transformation|GetActorLocation) "0, 0, 0" 1.0 1.0 0.0 0 0 0)
          (Utilities|FlowControl|Delay 0.2)
          (Actor|DestroyActor))))))

(event EventBeginPlay
  (Variables|Default|SetStartingZ (.z (Transformation|GetActorLocation))))

(event Collision|EventActorBeginOverlap
  (params (OtherActor :type Actor%20Object%20Reference)))

(event EventTick
  (params (DeltaSeconds :type Float%20%28single-precision%29))
  (bind _returnvalue (Transformation|GetActorLocation))
  (Transformation|SetWorldLocation (Variables|Default|GetSphere) (Math|Vector|MakeVector (.x _returnvalue) (.y _returnvalue) (+ (.z _returnvalue) (* (Variables|Default|GetRateOfMotion) (Variables|Default|GetDirection)))) false false)
  (Math|Integer|IncrementInt (Variables|Default|GetAcceleration)))

(fn ConstructionScript)