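; AI controller for Shade enemies that runs the behavior tree supplied by the possessed BP_Shade_Base.
; Each tick it mirrors the Shade's IsInPaint flag to the blackboard, damaging it while in paint and unpossessing once health runs out.
; Perception writes sighted actors to TargetActor and other stimuli to TargetLocation.
; Walk, Run and Alerted events drive movement and alert state; SetPassive is empty, and older overlap and sight logic is disconnected.
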(event OnTargetPerceptionUpdated(AIPerception)
  (params (Actor :type Actor%20Object%20Reference) (Stimulus :type AI%20Stimulus%20Structure))
  ;[1 1 1] Sensing Player
  (bind _returnvalue (Class|AIPerceptionSystem|GetSenseClassforStimulus Stimulus))
  (if (== _returnvalue "/Script/AIModule.AISense_Sight")
    (Variables|Default|SetTargetActor Actor)
    (AI|Components|Blackboard|SetValueasObject (Variables|Default|GetBlackboard) (Utilities|Name|MakeLiteralName "TargetActor") (Variables|Default|GetTargetActor))
    (else
      (AI|Components|Blackboard|SetValueasVector (Variables|Default|GetBlackboard) (Utilities|Name|MakeLiteralName "TargetLocation") (.StimulusLocation (Utilities|Struct|BreakAIStimulus Stimulus))))))

(event Custom|Walk
  ;[1 1 1] Movement
  (Default|Walk (Variables|Default|GetShade)))

(event Custom|Run
  ;[1 1 1] Movement
  (Default|Run (Variables|Default|GetShade)))

(event Custom|Alerted
  ;[1 1 1] Alerted States
  (AI|Components|Blackboard|SetValueasBool (AI|GetBlackboard 0) (Utilities|Name|MakeLiteralName "IsAlerted") true))

(event Custom|SetPassive
  ;[1 1 1] Alerted States
)

(event EventBeginPlay
  ;[1 1 1] Set Up
  (bind _asbp_shade_base (Utilities|Casting|CastToBP_Shade_Base (Pawn|GetControlledPawn)))
  (Variables|Default|SetShade _asbp_shade_base))

(event EventTick
  (params (DeltaSeconds :type Float%20%28single-precision%29))
  (bind _shade (Variables|Default|GetShade))
  ;[1 1 1] Check for Overlapping Paint Spheres
  (Utilities|FlowControl|Sequence
    (:then_0
      (if (Variables|/Game/Blueprints/Blueprints/Shades/BP_Shade_Base.BP_Shade_Base_C|GetisInPaint (Variables|Default|GetShade))
        (AI|Components|Blackboard|SetValueasBool (Variables|Default|GetBlackboard) (Utilities|Name|MakeLiteralName "IsInPaint") true)
        (if (<= (Variables|/Game/Blueprints/Blueprints/Shades/BP_Shade_Base.BP_Shade_Base_C|GetHealth _shade) 0.0)
          (Pawn|UnPossess)
          (else
            (Default|Damage _shade)))
        (else
          (AI|Components|Blackboard|SetValueasBool (Variables|Default|GetBlackboard) (Utilities|Name|MakeLiteralName "IsInPaint") false))))))

(event EventPossess
  (params (PossessedPawn :type Pawn%20Object%20Reference))
  ;[1 1 1] Running Behavior Tree
  (bind _asbp_shade_base (Utilities|Casting|CastToBP_Shade_Base PossessedPawn))
  (bind _output_get (Variables|Default|SetShade _asbp_shade_base))
  (AI|RunBehaviorTree (Variables|/Game/Blueprints/Blueprints/Shades/BP_Shade_Base.BP_Shade_Base_C|GetBehaviorTree _output_get)))

(fn ConstructionScript)