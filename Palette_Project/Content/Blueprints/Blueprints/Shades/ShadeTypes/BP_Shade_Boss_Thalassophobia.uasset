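; Thalassophobia boss Shade, a fishing-themed encounter that runs a behavior tree once started and ends when its health runs out.
; Each reel-in moves it forward along its starting facing; the third teleports it, sets the Blackboard "Caught" flag and loops a flop animation.
; Its spit attack spawns a shade ball above randomly picked fishing reel positions.
; Death notifies the easel pawn and destroys the black-and-white reference actor.
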(event Custom|ReeledIn
  (bind _startingforwardvector (Variables|Default|GetStartingForwardVector))
  (bind _capsulecomponent (Variables|Default|GetCapsuleComponent))
  (bind _returnvalue (Transformation|GetWorldLocation _capsulecomponent))
  (bind _returnvalue_2 (* _startingforwardvector 3e+02))
  (bind _returnvalue_3 (+ _returnvalue _returnvalue_2))
  (bind _result (Math|Integer|IncrementInt (Variables|Default|GetReeledInStage))
    (:%20%20
      (switch int _result
        (:1
          (AI|AIMoveTo self _returnvalue_3 0 5.0 false :!label _label))
        (:2
          (goto _label))
        (:3
          (AI|AIMoveTo self _returnvalue_3 0 5.0 false
            (:OnSuccess
              (Transformation|SetWorldLocation (Variables|Default|GetCapsuleComponent) (Transformation|GetActorLocation (Variables|Default|GetTeleporter)) false false)
              (AI|Components|Blackboard|SetValueasBool (AI|GetBlackboard (Pawn|GetController)) (Utilities|Name|MakeLiteralName "Caught") true)
              (Utilities|FlowControl|Delay 0.5)
              (Components|Animation|PlayAnimation (Variables|Character|GetMesh) "/Game/Assets/Characters/Shades/Boss_Thalassaphobia/Animations/Thalassophobia_FlopCycle.Thalassophobia_FlopCycle" true))))))))

(event Custom|EventSpitFishingPole
  (bind _fishingreelactors (Variables|Default|GetFishingReelActors))
  (bind _returnvalue (Utilities|Array|Length _fishingreelactors))
  (bind _returnvalue_2 (- _returnvalue 1))
  (bind _returnvalue_3 (Math|Random|RandomIntegerinRange 0 _returnvalue_2))
  (bind _output (Utilities|Array|Get(acopy) _fishingreelactors _returnvalue_3))
  (bind _returnvalue_4 (Transformation|GetActorLocation _output))
  (Components|Animation|PlayAnimation (Variables|Character|GetMesh) "/Game/Assets/Characters/Shades/Boss_Thalassaphobia/Animations/Thalassophobia_SpitAttack.Thalassophobia_SpitAttack" false)
  (Game|SpawnActorfromClass "/Game/Blueprints/Blueprints/Shades/BP_PhysicsObject_ShadeBall.BP_PhysicsObject_ShadeBall_C" (Math|Transform|MakeTransform (Math|Vector|MakeVector (.x _returnvalue_4) (.y _returnvalue_4) (+ (.z _returnvalue_4) 1e+03))) "AlwaysSpawn" 0 -1.0 0)
  (Utilities|FlowControl|Delay 2.0)
  (Components|Animation|SetAnimationMode (Variables|Character|GetMesh) "AnimationBlueprint"))

(event EventBeginPlay
  (bind _capsulecomponent (Variables|Default|GetCapsuleComponent))
  (Variables|Default|SetStartingPosition (Transformation|GetWorldLocation _capsulecomponent))
  (Variables|Default|SetStartingForwardVector (Math|Vector|GetForwardVector (Transformation|GetWorldRotation _capsulecomponent)))
  (|CallParentFunction))

(event Collision|EventActorBeginOverlap
  (params (OtherActor :type Actor%20Object%20Reference)))

(event EventTick
  (params (DeltaSeconds :type Float%20%28single-precision%29))
  (|CallParentFunction DeltaSeconds)
  (if (<= (Variables|Default|GetHealth) 0.0)
    (Utilities|FlowControl|DoOnce false
      (:Completed
        (CallFunction|BossEncounterEnd)))))

(event EventBossEncounterStart
  (Variables|Default|SetBehaviorTree "/Game/Blueprints/Blueprints/Shades/BehaviorTrees/BP_Boss_Thalassophobia_BT.BP_Boss_Thalassophobia_BT"))

(event EventBossEncounterEnd
  (bind _asbp_pawn_easel (Utilities|Casting|CastToBP_Pawn_Easel (Game|Player|GetPlayerPawn 0)))
  (Default|BossEncounterEnded _asbp_pawn_easel)
  (Actor|DestroyActor (Variables|Default|GetBlackAndWhiteReference)))

(fn ConstructionScript
  (|CallParentFunction))