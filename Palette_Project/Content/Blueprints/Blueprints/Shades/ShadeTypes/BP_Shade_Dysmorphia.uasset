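; BP_Shade_Dysmorphia is a Shade enemy variant that stays invisible unless it is standing in paint.
; BeginPlay hides the mesh and ColorInColors component and sets the run speed before calling the parent.
; Each tick toggles both components' visibility from IsInPaint, runs parent logic, and once Health reaches zero notifies its event volume a single time that the encounter is defeated.
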(event EventBeginPlay
  (Rendering|SetVisibility (Variables|Character|GetMesh) false false)
  (Rendering|SetVisibility (Variables|Default|GetColorInColors) false false)
  (Variables|Default|SetSpeed_Run 8e+02)
  (|CallParentFunction))

(event Collision|EventActorBeginOverlap
  (params (OtherActor :type Actor%20Object%20Reference)))

(event EventTick
  (params (DeltaSeconds :type Float%20%28single-precision%29))
  (bind _mesh (Variables|Character|GetMesh))
  (bind _colorincolors (Variables|Default|GetColorInColors))
  (Utilities|FlowControl|Sequence
    (:then_0
      (if (Variables|Default|GetisInPaint)
        (Rendering|SetVisibility _mesh true false)
        (Rendering|SetVisibility _colorincolors true false)
        (else
          (Rendering|SetVisibility _mesh false false)
          (Rendering|SetVisibility _colorincolors false false)))
      (|CallParentFunction DeltaSeconds))
    (:then_1
      (if (<= (Variables|Default|GetHealth) 0.0)
        (Utilities|FlowControl|DoOnce false
          (:Completed
            (Default|EncounterDefeated (Variables|Default|GetEventVolumeReference))))))))

(fn ConstructionScript
  (|CallParentFunction))