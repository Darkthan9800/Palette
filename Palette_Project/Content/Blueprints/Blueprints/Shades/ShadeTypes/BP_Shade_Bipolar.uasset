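; Bipolar Shade, a shade variant whose vulnerable color changes at random between blue, red and yellow.
; A self-restarting loop waits a few seconds, picks a weakness index, and sets the matching color parameter on its ColorInColors component.
; While possessed, Tick copies the easel pawn palette's frozen state into the controller's Blackboard before running parent Tick logic.
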(event Custom|SwitchVulnerability
  (bind _colorincolors (Variables|Default|GetColorInColors))
  (bind _output_get (Variables|Default|SetWeaknessColor (Math|Random|RandomIntegerinRange 0 2)))
  (switch int _output_get
    (:0
      (Effects|Components|ParticleSystem|SetColorParameter _colorincolors "ShadeVulnerableColor" "(R=0.000000,G=0.000000,B=1.000000,A=1.000000)"))
    (:1
      (Effects|Components|ParticleSystem|SetColorParameter _colorincolors "ShadeVulnerableColor" "(R=1.000000,G=0.000000,B=0.000000,A=1.000000)"))
    (:2
      (Effects|Components|ParticleSystem|SetColorParameter _colorincolors "ShadeVulnerableColor" "(R=1.000000,G=1.000000,B=0.000000,A=1.000000)")))
  (CallFunction|SwitchDelay))

(event Custom|Switch%20Delay
  (Utilities|FlowControl|RetriggerableDelay (Math|Random|RandomFloatinRange 3.0 5.0))
  (CallFunction|SwitchVulnerability))

(event EventBeginPlay
  (bind _asbp_pawn_easel (Utilities|Casting|CastToBP_Pawn_Easel (Game|Player|GetPlayerPawn 0)))
  (Variables|Default|SetAs%20BP%20Pawn%20Easel _asbp_pawn_easel)
  (CallFunction|SwitchDelay)
  (|CallParentFunction))

(event Collision|EventActorBeginOverlap
  (params (OtherActor :type Actor%20Object%20Reference))
  (|CallParentFunction OtherActor) ; This node is disabled and will not be called.\nDrag off pins to build functionality.
)

(event EventTick
  (params (DeltaSeconds :type Float%20%28single-precision%29))
  (if (Variables|Default|GetIsPossessed)
    (AI|Components|Blackboard|SetValueasBool (AI|GetBlackboard (Pawn|GetController)) (Utilities|Name|MakeLiteralName "IsPaletteFrozen") (Variables|/Game/Blueprints/Blueprints/BP_Pawn_Palette.BP_Pawn_Palette_C|GetIsFrozen (Variables|/Game/Blueprints/Blueprints/BP_Pawn_Easel.BP_Pawn_Easel_C|GetPaletteReference (Variables|Default|GetAs%20BP%20Pawn%20Easel))))
    (|CallParentFunction DeltaSeconds)))

(event EventUnpossessed
  (params (OldController :type Controller%20Object%20Reference))
  (Variables|Default|SetIsPossessed false))

(fn ConstructionScript
  (|CallParentFunction))