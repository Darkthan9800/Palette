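; Palette pawn that follows and turns toward the mouse cursor's hit point in the world, starting beside the easel.
; BeginPlay uses the game mode's player count to disable its camera and hide the cursor marker for one player, enabling both otherwise.
; Tick traces under player 0's cursor, moving the pawn via MovementInterpolation and aligning CursorToWorld to the surface normal.
; MovementInterpolation contains per-axis FInterpTo easing, shown unconnected to any output.
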(event EventBeginPlay
  (bind _easelreference (Variables|Default|GetEaselReference))
  (bind _camera1 (Variables|Default|GetCamera1))
  (bind _cursortoworld (Variables|Default|GetCursorToWorld))
  (bind _returnvalue (Transformation|GetActorLocation _easelreference))
  ;[1 1 1] Event Begin Play
  (bind _aspalette_gamemode (Utilities|Casting|CastToPalette_Gamemode (Game|GetGameMode)))
  (bind _output_get (Variables|Default|SetPalette_Gamemode _aspalette_gamemode))
  (bind _returnvalue_2 (Class|GameModeBase|GetNumPlayers _output_get))
  (if (== _returnvalue_2 1)
    (Components|Activation|Deactivate _camera1)
    (Rendering|SetVisibility _cursortoworld false false)
    (else
      (Components|Activation|Activate _camera1 false)
      (Rendering|SetVisibility _cursortoworld true false)))
  ;;[0 1 0.06035] Beginning Location
  (Transformation|SetActorLocation (Math|Vector|MakeVector (.x _returnvalue) (+ (.y _returnvalue) 1e+02) (.z _returnvalue)) false false)
  (Input|EnableInput (Game|GetPlayerController 0)))

(event EventTick
  (params (DeltaSeconds :type Float%20%28single-precision%29))
  (bind _returnvalue (Game|GetPlayerController 0))
  (bind _hitresult (Game|Player|GetHitResultUnderCursorbyChannel _returnvalue "TraceTypeQuery1" true))
  (bind (_bblockinghit _binitialoverlap _time _distance _location _impactpoint _normal _impactnormal) (Collision|BreakHitResult _hitresult))
  (bind _returnvalue_2 (Math|Vector|MakeVector (.x _location) (.y _location) (.z _location)))
  ;[1 1 1] Event Tick
  (Variables|Default|SetDeltaSeconds DeltaSeconds)
  ;;[0 1 0.06268] Set Location and Rotation
  (Transformation|SetActorLocationAndRotation (|MovementInterpolation (.x _location) (.y _location) (.z _location)) (Class|KismetMathLibrary|RInterptoConstant (Transformation|GetActorRotation) (Math|Conversions|RotationFromXVector (Math|Vector|GetUnitDirection(Vector) (Transformation|GetActorLocation) _returnvalue_2)) (Variables|Default|GetDeltaSeconds) 5e+02))
  (Transformation|SetWorldLocationAndRotation (Variables|Default|GetCursorToWorld) _returnvalue_2 (Math|Rotator|MakeRotationfromAxes (Math|Vector|MakeVector (.x _impactnormal) (.y _impactnormal) (.z _impactnormal)) "0, 0, 0" "0, 0, 0") false false))

(fn ConstructionScript)