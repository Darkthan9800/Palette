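; BP_PaintBucket is a floating, glowing paint bucket actor in one of five colors.
; BeginPlay keeps the set color when PaintUnlock is true, otherwise picks randomly from blue, red or yellow, then applies it through a dynamic material and matching point light.
; It enables custom depth with a stencil value on the mesh.
; A timeline drives Height, which Tick adds, scaled, to the bucket's Z each frame without delta-time scaling.
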(event EventBeginPlay
  (bind _paintbucket (Variables|Default|GetPaintBucket))
  (Utilities|FlowControl|Sequence
    (:then_0
      (Rendering|SetRenderCustomDepth _paintbucket true)
      (Rendering|SetCustomDepthStencilValue _paintbucket 1))
    (:then_1
      (bind _returnvalue (Rendering|Material|CreateDynamicMaterialInstance (Rendering|Material|GetMaterial (Variables|Default|GetPaintBucket) 0) "None" "None" :!class /Script/Engine.KismetMaterialLibrary))
      (Variables|Default|SetDynamicPaintMaterial _returnvalue)
      (if (Variables|Default|GetPaintUnlock?)
        (switch int (Variables|Default|GetPaintBucketColor)
          (:0
            (Rendering|Material|SetVectorParameterValue (Variables|Default|GetDynamicPaintMaterial) "PaintBucketColor" "(R=0.000000,G=0.000000,B=1.000000,A=1.000000)" :!class /Script/Engine.MaterialInstanceDynamic)
            (Variables|Default|SetPaintBucketColorValues "(R=0.000000,G=0.067130,B=1.000000,A=1.000000)"))
          (:1
            (Rendering|Material|SetVectorParameterValue (Variables|Default|GetDynamicPaintMaterial) "PaintBucketColor" "(R=1.000000,G=0.000000,B=0.000000,A=1.000000)" :!class /Script/Engine.MaterialInstanceDynamic)
            (Variables|Default|SetPaintBucketColorValues "(R=1.000000,G=0.057804,B=0.000000,A=1.000000)"))
          (:2
            (Rendering|Material|SetVectorParameterValue (Variables|Default|GetDynamicPaintMaterial) "PaintBucketColor" "(R=1.000000,G=1.000000,B=0.000000,A=1.000000)" :!class /Script/Engine.MaterialInstanceDynamic)
            (Variables|Default|SetPaintBucketColorValues "(R=1.000000,G=0.946557,B=0.000000,A=1.000000)"))
          (:3
            (Rendering|Material|SetVectorParameterValue (Variables|Default|GetDynamicPaintMaterial) "PaintBucketColor" "(R=1.000000,G=0.354000,B=0.000000,A=1.000000)" :!class /Script/Engine.MaterialInstanceDynamic)
            (Variables|Default|SetPaintBucketColorValues "(R=1.000000,G=0.415300,B=0.000000,A=1.000000)"))
          (:4
            (Rendering|Material|SetVectorParameterValue (Variables|Default|GetDynamicPaintMaterial) "PaintBucketColor" "(R=0.311502,G=0.000000,B=1.000000,A=1.000000)" :!class /Script/Engine.MaterialInstanceDynamic)
            (Variables|Default|SetPaintBucketColorValues "(R=0.342295,G=0.000000,B=1.000000,A=1.000000)")))
        (else
          (bind _output_get (Variables|Default|SetPaintBucketColor (Math|Random|RandomIntegerinRange 0 2)))
          (switch int _output_get
            (:0
              (Rendering|Material|SetVectorParameterValue (Variables|Default|GetDynamicPaintMaterial) "PaintBucketColor" "(R=0.000000,G=0.000000,B=1.000000,A=1.000000)" :!class /Script/Engine.MaterialInstanceDynamic)
              (Variables|Default|SetPaintBucketColorValues "(R=0.000000,G=0.067130,B=1.000000,A=1.000000)"))
            (:1
              (Rendering|Material|SetVectorParameterValue (Variables|Default|GetDynamicPaintMaterial) "PaintBucketColor" "(R=1.000000,G=0.000000,B=0.000000,A=1.000000)" :!class /Script/Engine.MaterialInstanceDynamic)
              (Variables|Default|SetPaintBucketColorValues "(R=1.000000,G=0.057804,B=0.000000,A=1.000000)"))
            (:2
              (Rendering|Material|SetVectorParameterValue (Variables|Default|GetDynamicPaintMaterial) "PaintBucketColor" "(R=1.000000,G=1.000000,B=0.000000,A=1.000000)" :!class /Script/Engine.MaterialInstanceDynamic)
              (Variables|Default|SetPaintBucketColorValues "(R=1.000000,G=0.946557,B=0.000000,A=1.000000)"))
            (:3
              (Rendering|Material|SetVectorParameterValue (Variables|Default|GetDynamicPaintMaterial) "PaintBucketColor" "(R=1.000000,G=0.354000,B=0.000000,A=1.000000)" :!class /Script/Engine.MaterialInstanceDynamic)
              (Variables|Default|SetPaintBucketColorValues "(R=1.000000,G=0.415300,B=0.000000,A=1.000000)"))
            (:4
              (Rendering|Material|SetVectorParameterValue (Variables|Default|GetDynamicPaintMaterial) "PaintBucketColor" "(R=0.311501,G=0.000000,B=1.000000,A=1.000000)" :!class /Script/Engine.MaterialInstanceDynamic)
              (Variables|Default|SetPaintBucketColorValues "(R=0.342295,G=0.000000,B=1.000000,A=1.000000)"))))))
    (:then_2
      (Rendering|Material|SetMaterial (Variables|Default|GetPaintBucket) 0 (Variables|Default|GetDynamicPaintMaterial)))
    (:then_3
      (Rendering|Components|Light|SetLightColor (Variables|Default|GetPointLight) (Variables|Default|GetPaintBucketColorValues) true))
    (:then_4
      (bind _newtrack_0 (Timeline|FloatUpAndDown PlayFromStart)
        (:Update
          (Variables|Default|SetHeight _newtrack_0))))))

(event Collision|EventActorBeginOverlap
  (params (OtherActor :type Actor%20Object%20Reference)))

(event EventTick
  (params (DeltaSeconds :type Float%20%28single-precision%29))
  (bind _paintbucket (Variables|Default|GetPaintBucket))
  (bind _returnvalue (Transformation|GetWorldLocation _paintbucket))
  (Transformation|SetWorldLocation (Variables|Default|GetPaintBucket) (Math|Vector|MakeVector (.x _returnvalue) (.y _returnvalue) (+ (.z _returnvalue) (* (Variables|Default|GetHeight) 2.0))) false false))

(fn ConstructionScript)