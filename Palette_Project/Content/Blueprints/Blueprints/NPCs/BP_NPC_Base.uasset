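; Base NPC Blueprint that shows paged dialogue on interaction and enables custom depth stencil on its mesh.
; Each Interact advances through NPCText in a UI_Dialogue widget with two portrait images, then closes it and restores Animation Blueprint mode after the last line.
; QuestStage 1 calls the empty QuestStage01 event instead of the default dialogue.
; Ending overlap removes the widget without resetting the dialogue index or talking flag.
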(event Custom|QuestStage01)

(event EventBeginPlay
  (bind _mesh (Variables|Character|GetMesh))
  (Rendering|SetRenderCustomDepth _mesh true)
  (Rendering|SetCustomDepthStencilValue _mesh 1)
  (Variables|Default|SetNumberOfStages (+ (Utilities|Array|Length (Variables|Default|GetNPCText)) 1)))

(event Collision|EventActorBeginOverlap
  (params (OtherActor :type Actor%20Object%20Reference)))

(event EventTick
  (params (DeltaSeconds :type Float%20%28single-precision%29)))

(event EventInteract
  (Variables|Default|SetIsTalking true)
  (switch int (Variables|Default|GetQuestStage)
    (:Default
      ;[1 1 1] Stage 01
      (if (and (> (Variables|Default|GetNumberOfStages) (+ (Variables|Default|GetDialogueStage) 1)) (== (Variables|Default|GetDialogueStage) 0)) :!label _label
        (bind _returnvalue (UserInterface|CreateWidget "/Game/Blueprints/Blueprints/UI/UI_Dialogue.UI_Dialogue_C" (Game|GetPlayerController 0) :!label _label_2))
        (bind _output_get (Variables|Default|SetDialogueWidget _returnvalue))
        (UserInterface|Viewport|AddtoViewport _output_get 0)
        (Variables|/Game/Blueprints/Blueprints/UI/UI_Dialogue.UI_Dialogue_C|SetDialogue_Other (Variables|Default|GetDialogueWidget) (Utilities|Array|Get(acopy) (Variables|Default|GetNPCText) (Variables|Default|GetDialogueStage)) :!label _label_3)
        (Variables|/Game/Blueprints/Blueprints/UI/UI_Dialogue.UI_Dialogue_C|SetEaselDialogueImage (Variables|Default|GetDialogueWidget) (Variables|Default|GetEaselDialogueImage))
        (Variables|/Game/Blueprints/Blueprints/UI/UI_Dialogue.UI_Dialogue_C|SetOtherActorDialogueImage (Variables|Default|GetDialogueWidget) (Variables|Default|GetOtherActorDialogueImage))
        (Math|Integer|IncrementInt (Variables|Default|GetDialogueStage))
        (else
          (if (> (Variables|Default|GetDialogueStage) 0)
            (if (>= (+ (Variables|Default|GetDialogueStage) 1) (Variables|Default|GetNumberOfStages))
              _
              (else
                (goto _label_3)))
            (else
              (Utilities|IsValid (Variables|Default|GetDialogueWidget)
                (:Is%20Valid
                  _)
                (:Is%20Not%20Valid
                  (goto _label_2)))))
          (Widget|RemovefromParent (Variables|Default|GetDialogueWidget))
          (Variables|Default|SetDialogueWidget 0)
          (Variables|Default|SetDialogueStage 0)
          (Variables|Default|SetIsTalking false)
          (Components|Animation|SetAnimationMode (Variables|Character|GetMesh) "AnimationBlueprint"))))
    (:0
      (goto _label))
    (:1
      (CallFunction|QuestStage01))))

(event Collision|EventActorEndOverlap
  (params (OtherActor :type Actor%20Object%20Reference))
  (Utilities|IsValid (Variables|Default|GetDialogueWidget)
    (:Is%20Valid
      (Widget|RemovefromParent (Variables|Default|GetDialogueWidget))
      (Variables|Default|SetDialogueWidget 0))))

(fn ConstructionScript)