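; BP_NPC_Snail01 is a snail NPC Blueprint that switches its mesh to a looping talking animation when it starts talking.
; Tick polls IsTalking and uses a DoOnce, reset while not talking, so the animation starts once per talking session.
; The parent Tick is chained after that DoOnce, so it runs only on that first talking frame.
; Nothing here restores another animation when talking ends.
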(event EventBeginPlay
  (|CallParentFunction) ; This node is disabled and will not be called.\nDrag off pins to build functionality.
)

(event Collision|EventActorBeginOverlap
  (params (OtherActor :type Actor%20Object%20Reference))
  (|CallParentFunction OtherActor) ; This node is disabled and will not be called.\nDrag off pins to build functionality.
)

(event EventTick
  (params (DeltaSeconds :type Float%20%28single-precision%29))
  (if (Variables|Default|GetIsTalking)
    (Utilities|FlowControl|DoOnce false :!label _label
      (:Completed
        (Components|Animation|PlayAnimation (Variables|Character|GetMesh) "/Game/Assets/Characters/NPCs/BeachLevel_Snails/Animations/CoolSnail/CoolSnail_Talking.CoolSnail_Talking" true)
        (|CallParentFunction DeltaSeconds)))
    (else
      (goto _label Reset))))

(fn ConstructionScript
  (|CallParentFunction))