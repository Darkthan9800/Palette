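; BP_NPC_Ghost_ColoredIn is a ghost NPC Blueprint that animates its mesh vertically, apparently as a floating effect.
; A timeline started on BeginPlay writes its track value to Height, and Tick adds double that to the mesh's world Z each frame.
; The offset accumulates without delta-time scaling, so movement depends on frame rate.
; Parent BeginPlay is wired to the timeline's Update, so it runs on every update.
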(event EventBeginPlay
  (bind _newtrack_0 (Timeline|Timeline_0 PlayFromStart)
    (:Update
      (Variables|Default|SetHeight _newtrack_0)
      (|CallParentFunction))))

(event Collision|EventActorBeginOverlap
  (params (OtherActor :type Actor%20Object%20Reference))
  (|CallParentFunction OtherActor) ; This node is disabled and will not be called.\nDrag off pins to build functionality.
)

(event EventTick
  (params (DeltaSeconds :type Float%20%28single-precision%29))
  (bind _mesh (Variables|Character|GetMesh))
  (bind _returnvalue (Transformation|GetWorldLocation _mesh))
  (Transformation|SetWorldLocation _mesh (Math|Vector|MakeVector (.x _returnvalue) (.y _returnvalue) (+ (.z _returnvalue) (* (Variables|Default|GetHeight) 2.0))) false false)
  (|CallParentFunction DeltaSeconds))

(fn ConstructionScript
  (|CallParentFunction))