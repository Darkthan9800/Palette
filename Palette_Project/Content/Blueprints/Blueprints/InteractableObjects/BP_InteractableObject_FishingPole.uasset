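; Interactable fishing pole that calls ReeledIn on a referenced Thalassophobia object when used while clean.
; Tick marks it not clean while a BP_Shade_PaintObject overlaps its Sphere.
; Interacting while painted briefly shows a dialogue widget through a retriggerable delay.
; A DoOnce gates activation, and a separate Delay event resets it after DelayTime.
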(event Custom|Delay
  (Utilities|FlowControl|Delay (Variables|Default|GetDelayTime))
  (Utilities|FlowControl|DoOnce false) ; enters at Reset
)

(event EventBeginPlay
  (|CallParentFunction) ; This node is disabled and will not be called.\nDrag off pins to build functionality.
)

(event Collision|EventActorBeginOverlap
  (params (OtherActor :type Actor%20Object%20Reference))
  (|CallParentFunction OtherActor) ; This node is disabled and will not be called.\nDrag off pins to build functionality.
)

(event EventTick
  (params (DeltaSeconds :type Float%20%28single-precision%29))
  (Utilities|IsValid (Utilities|Array|Get(acopy) (Collision|GetOverlappingActors (Variables|Default|GetSphere) "/Game/Blueprints/Blueprints/BP_Shade_PaintObject.BP_Shade_PaintObject_C" :!class /Script/Engine.PrimitiveComponent))
    (:Is%20Valid
      (Variables|Default|SetClean false))
    (:Is%20Not%20Valid
      (Variables|Default|SetClean true)))
  (|CallParentFunction DeltaSeconds))

(event EventInteract
  (bind _dialoguewidget (Variables|Default|GetDialogueWidget))
  (if (Variables|Default|GetClean)
    (Utilities|FlowControl|DoOnce false
      (:Completed
        (Development|PrintString "Activated")
        (Default|Reeledin (Variables|Default|GetThalassophobiaReference))))
    (else
      (Rendering|SetVisibility _dialoguewidget true false)
      (Utilities|FlowControl|RetriggerableDelay 2.0)
      (Rendering|SetVisibility _dialoguewidget false false))))

(fn ConstructionScript
  (|CallParentFunction))