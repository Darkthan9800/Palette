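; BP_PaintObject is a paint blob actor that makes noise for AI hearing and clears away nearby BP_Shade_PaintObject actors.
; On BeginPlay it reports a noise event, plays one of four random goop sounds, then destroys shade paint objects found by a sphere overlap.
; The ChangedPaintColor event repeats the noise report and clearing with a smaller radius and no sound.
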(event Custom|ChangedPaintColor
  (bind _returnvalue (Transformation|GetActorLocation))
  (Class|AISenseHearing|ReportNoiseEvent _returnvalue 2.0 self 1e+03 "None")
  (bind _outactors (Collision|SphereOverlapActors _returnvalue 1e+02 (Utilities|Array|MakeArray "ObjectTypeQuery2") "/Game/Blueprints/Blueprints/BP_Shade_PaintObject.BP_Shade_PaintObject_C"))
  (for _array_element _outactors
    (Actor|DestroyActor _array_element)))

(event EventBeginPlay
  (bind _returnvalue (Transformation|GetActorLocation))
  (Class|AISenseHearing|ReportNoiseEvent _returnvalue 2.0 self 1e+03 "None")
  (switch int (Math|Random|RandomIntegerinRange 0 3)
    (:0
      (Audio|SpawnSoundatLocation "/Game/Assets/Sounds/GoopSounds01.GoopSounds01" _returnvalue "0, 0, 0" 1.0 1.0 0.0 0 0))
    (:1
      (Audio|SpawnSoundatLocation "/Game/Assets/Sounds/GoopSounds02.GoopSounds02" _returnvalue "0, 0, 0" 1.0 1.0 0.0 0 0))
    (:2
      (Audio|SpawnSoundatLocation "/Game/Assets/Sounds/GoopSounds03.GoopSounds03" _returnvalue "0, 0, 0" 1.0 1.0 0.0 0 0))
    (:3
      (Audio|SpawnSoundatLocation "/Game/Assets/Sounds/GoopSounds04.GoopSounds04" _returnvalue "0, 0, 0" 1.0 1.0 0.0 0 0)))
  (bind _outactors (Collision|SphereOverlapActors (Transformation|GetActorLocation) 2e+02 (Utilities|Array|MakeArray "ObjectTypeQuery2") "/Game/Blueprints/Blueprints/BP_Shade_PaintObject.BP_Shade_PaintObject_C"))
  (for _array_element _outactors
    (Actor|DestroyActor _array_element)))

(event Collision|EventActorBeginOverlap
  (params (OtherActor :type Actor%20Object%20Reference)))

(event EventTick
  (params (DeltaSeconds :type Float%20%28single-precision%29)))

(fn ConstructionScript)