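; BP_EventVolume is a trigger volume that closes referenced doors when the player's BP_Pawn_Easel enters, and reopens them after an encounter is defeated.
; Overlap waits through a short delay, then a DoOnce closes every entry in DoorReferences, so the lock-in happens only once.
; The EncounterDefeated event, which nothing in this graph calls, waits briefly and then opens the same doors.
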(event Custom|EncounterDefeated
  (Utilities|FlowControl|Delay 1.0)
  (for _array_element (Variables|Default|GetDoorReferences)
    (Default|Open _array_element)))

(event EventBeginPlay)

(event Collision|EventActorBeginOverlap
  (params (OtherActor :type Actor%20Object%20Reference))
  (Utilities|Casting|CastToBP_Pawn_Easel OtherActor)
  (Utilities|FlowControl|Delay 2.0)
  (Utilities|FlowControl|DoOnce false
    (:Completed
      (for _array_element (Variables|Default|GetDoorReferences)
        (Default|Close _array_element)))))

(event EventTick
  (params (DeltaSeconds :type Float%20%28single-precision%29)))

(fn ConstructionScript)