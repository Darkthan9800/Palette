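; Paintable static object that the palette pawn can splat paint onto or absorb paint from at runtime.
; BeginPlay creates a render target and feeds it, with the object's textures, into dynamic canvas and eraser materials, plus a splat brush material.
; Every Tick it runs a complex trace from the pawn's paint arrow, converts self-hits to UVs, and draws brush or eraser into the target with randomized size and rotation.
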(event EventTick
  (params (DeltaSeconds :type Float%20%28single-precision%29))
  (bind _pawn_palette (Variables|Default|GetPawn_Palette))
  (bind _pawn_palette_2 (Variables|Default|GetPawn_Palette))
  (bind _paintarrow (Variables|/Game/Blueprints/Blueprints/Pawn_Palette.Pawn_Palette_C|GetPaintArrow _pawn_palette_2))
  (bind _returnvalue (Transformation|GetWorldLocation _paintarrow))
  (Utilities|FlowControl|Sequence
    (:then_0
      ;[1 1 1] Find Paint Location / Render Target
      (Variables|Default|SetTargetBrushSize (- (Variables|Default|GetCurrentBrushSize) (Math|Random|RandomFloatinRange 0.0 (/ (Variables|Default|GetCurrentBrushSize) 2.0))))
      (bind (_outhit _returnvalue_2) (Collision|LineTraceForObjects _returnvalue (+ _returnvalue (* (Math|Vector|GetForwardVector (Transformation|GetWorldRotation _paintarrow)) (Variables|Default|GetLineTraceDistance))) (Utilities|Array|MakeArray "ObjectTypeQuery1") true 0 "ForOneFrame" false))
      (if (== (.hitactor _outhit) self)
        (if _returnvalue_2
          (if (Variables|/Game/Blueprints/Blueprints/Pawn_Palette.Pawn_Palette_C|GetIsPainting (Variables|Default|GetPawn_Palette))
            (CallFunction|DrawBrush (Utilities|Array|Get(acopy) (Variables|/Game/Blueprints/Blueprints/Pawn_Palette.Pawn_Palette_C|GetPaint_Brushes _pawn_palette) (Variables|/Game/Blueprints/Blueprints/Pawn_Palette.Pawn_Palette_C|GetCurrentPaintColor_Index _pawn_palette)) (Variables|Default|GetTargetBrushSize) (.UV (Class|GameplayStatics|FindCollisionUV (Collision|MakeHitResult (.bblockinghit _outhit) (.binitialoverlap _outhit) (.time _outhit) (.distance _outhit) (.location _outhit) (.impactpoint _outhit) (.normal _outhit) (.impactnormal _outhit) (.physmat _outhit) (.hitactor _outhit) (.hitcomponent _outhit) (.hitbonename _outhit) (.hititem _outhit) (.faceindex _outhit) (.tracestart _outhit) (.traceend _outhit)))))
            (elif (Variables|/Game/Blueprints/Blueprints/Pawn_Palette.Pawn_Palette_C|GetIsAbsorbing (Variables|Default|GetPawn_Palette))
              (CallFunction|AbsorbBrush "/Game/Assets/Characters/Palette/Paint/Texture_EraserAlpha.Texture_EraserAlpha" (Variables|Default|GetTargetBrushSize) (.UV (Class|GameplayStatics|FindCollisionUV (Collision|MakeHitResult (.bblockinghit _outhit) (.binitialoverlap _outhit) (.time _outhit) (.distance _outhit) (.location _outhit) (.impactpoint _outhit) (.normal _outhit) (.impactnormal _outhit) (.physmat _outhit) (.hitactor _outhit) (.hitcomponent _outhit) (.hitbonename _outhit) (.hititem _outhit) (.faceindex _outhit) (.tracestart _outhit) (.traceend _outhit))))))))))))

(event EventBeginPlay
  (bind _rendertarget_size (Variables|Default|GetRenderTarget_Size))
  ;[1 1 1] Setup
  (Utilities|FlowControl|Sequence
    (:then_0
      ;;[1 1 1] Create Render Target / Brush Size
      (bind _returnvalue (Rendering|CreateRenderTarget2D _rendertarget_size _rendertarget_size "RTF_RGBA16f" "(R=0.000000,G=0.000000,B=0.000000,A=0.000000)"))
      (bind _output_get (Variables|Default|SetRenderTarget _returnvalue))
      (Rendering|ClearRenderTarget2D _output_get)
      (Variables|Default|SetCurrentBrushSize (Variables|Default|GetTargetBrushSize)))
    (:then_1
      ;;[1 1 1] Canvas Material
      (bind _returnvalue_2 (Rendering|Material|CreateDynamicMaterialInstance (Variables|Default|GetCanvasMaterial) "None" "None" :!class /Script/Engine.KismetMaterialLibrary))
      (Rendering|Material|SetTextureParameterValue _returnvalue_2 "RenderTarget" (Variables|Default|GetRenderTarget))
      (Rendering|Material|SetTextureParameterValue _returnvalue_2 "ObjectMaterial_Albedo" (Variables|Default|GetObjectTexture_Albedo))
      (Rendering|Material|SetTextureParameterValue _returnvalue_2 "ObjectMaterial_ChannelPack" (Variables|Default|GetObjectTexture_ChannelPack))
      (Rendering|Material|SetTextureParameterValue _returnvalue_2 "ObjectMaterial_Normals" (Variables|Default|GetObjectTexture_Normals))
      (bind _output_get_2 (Variables|Default|SetCanvas _returnvalue_2))
      (Rendering|Material|SetMaterial (Variables|Default|GetPaintableSurface) 0 _output_get_2))
    (:then_2
      ;;[1 1 1] Brush Material
      (bind _returnvalue_3 (Rendering|Material|CreateDynamicMaterialInstance "/Game/Assets/Characters/Palette/Paint/Mat_Splat.Mat_Splat" "None" "None" :!class /Script/Engine.KismetMaterialLibrary))
      (Variables|Default|SetBrushMaterial _returnvalue_3))
    (:then_3
      ;;[1 1 1] Eraser Material
      (bind _returnvalue_4 (Rendering|Material|CreateDynamicMaterialInstance "/Game/Assets/Characters/Palette/Paint/Mat_Eraser.Mat_Eraser" "None" "None" :!class /Script/Engine.KismetMaterialLibrary))
      (bind _output_get_3 (Variables|Default|SetEraserMaterial _returnvalue_4))
      (Rendering|Material|SetTextureParameterValue _output_get_3 "ObjectMaterial_Albedo" (Variables|Default|GetObjectTexture_Albedo))
      (Rendering|Material|SetScalarParameterValue _output_get_3 "Size" (Variables|Default|GetTargetBrushSize) :!class /Script/Engine.MaterialInstanceDynamic)
      (Rendering|Material|SetTextureParameterValue _output_get_3 "RenderTarget" (Variables|Default|GetRenderTarget)))))

(fn ConstructionScript)

(fn DrawBrush
  (params (BrushTexture :type Texture%202D%20Object%20Reference) (BrushSize :type Float%20%28single-precision%29) (DrawLocation :type Vector%202D%20Structure))
  (bind _targetbrushsize (Variables|Default|GetTargetBrushSize))
  (Utilities|FlowControl|Sequence
    (:then_0
      (Rendering|Material|SetTextureParameterValue (Variables|Default|GetBrushMaterial) "BrushTexture" BrushTexture))
    (:then_1
      (bind (_canvas _size _context) (Rendering|BeginDrawCanvastoRenderTarget (Variables|Default|GetRenderTarget)))
      (Canvas|DrawMaterial :self _canvas :RenderMaterial (Variables|Default|GetBrushMaterial) :ScreenPosition (- (* _size DrawLocation) (/ _targetbrushsize 2.0)) :ScreenSize (Math|Vector2D|MakeVector2D _targetbrushsize _targetbrushsize) :CoordinateSize "(X=1.000000,Y=1.000000)" :Rotation (Math|Random|RandomFloatinRange 0.0 3.6e+02) :PivotPoint "(X=0.500000,Y=0.500000)")
      (Rendering|EndDrawCanvastoRenderTarget _context))))

(fn AbsorbBrush
  (params (BrushTexture :type Texture%202D%20Object%20Reference) (BrushSize :type Float%20%28single-precision%29) (DrawLocation :type Vector%202D%20Structure))
  (bind _targetbrushsize (Variables|Default|GetTargetBrushSize))
  (Utilities|FlowControl|Sequence
    (:then_0
      (Rendering|Material|SetTextureParameterValue (Variables|Default|GetEraserMaterial) "BrushMask" BrushTexture))
    (:then_1
      (bind (_canvas _size _context) (Rendering|BeginDrawCanvastoRenderTarget (Variables|Default|GetRenderTarget)))
      (Canvas|DrawMaterial :self _canvas :RenderMaterial (Variables|Default|GetEraserMaterial) :ScreenPosition (- (* _size DrawLocation) (/ _targetbrushsize 2.0)) :ScreenSize (Math|Vector2D|MakeVector2D _targetbrushsize _targetbrushsize) :CoordinateSize "(X=1.000000,Y=1.000000)" :Rotation (Math|Random|RandomFloatinRange 0.0 3.6e+02) :PivotPoint "(X=0.500000,Y=0.500000)")
      (Rendering|EndDrawCanvastoRenderTarget _context))))