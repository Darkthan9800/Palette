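; Static world object whose surface the player can paint or absorb paint from, and that shade paint orbs can splat.
; BeginPlay creates a render target feeding canvas and eraser dynamic materials, and enables custom depth on the surface.
; Tick traces from the palette's arrow, converting hits to collision UVs to stamp size-jittered, randomly rotated brush or eraser materials into the target.
; ShadePaint traces from each unsplatted orb to stamp shade splats.
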(event Custom|ShadePaint
  (CallFunction|ShadePaintTrace))

(event EventTick
  (params (DeltaSeconds :type Float%20%28single-precision%29))
  (bind _pawn_palette (Variables|Default|GetPawn_Palette))
  (bind _paintarrow (Variables|/Game/Blueprints/Blueprints/BP_Pawn_Palette.BP_Pawn_Palette_C|GetPaintArrow _pawn_palette))
  (bind _returnvalue (Transformation|GetWorldLocation _paintarrow))
  ;[1 1 1] Find Paint Location / Render Target
  (Variables|Default|SetTargetBrushSize (- (Variables|Default|GetCurrentBrushSize) (Math|Random|RandomFloatinRange 0.0 (/ (Variables|Default|GetCurrentBrushSize) 2.0))))
  (bind (_outhit _returnvalue_2) (Collision|LineTraceForObjects _returnvalue (+ _returnvalue (* (Math|Vector|GetForwardVector (Transformation|GetWorldRotation _paintarrow)) (Variables|Default|GetLineTraceDistance))) (Utilities|Array|MakeArray "ObjectTypeQuery1") true 0 "None" false))
  (if (== (.hitactor _outhit) self)
    (if _returnvalue_2
      (if (and (Variables|/Game/Blueprints/Blueprints/BP_Pawn_Palette.BP_Pawn_Palette_C|GetIsPainting (Variables|Default|GetPawn_Palette)) (not (Variables|/Game/Blueprints/Blueprints/BP_Pawn_Easel.BP_Pawn_Easel_C|GetCurrentPaintEmpty (Variables|Default|GetPawnEasel))))
        (CallFunction|DrawBrushNew (Variables|Default|GetTargetBrushSize) (.UV (Class|GameplayStatics|FindCollisionUV (Collision|MakeHitResult (.bblockinghit _outhit) (.binitialoverlap _outhit) (.time _outhit) (.distance _outhit) (.location _outhit) (.impactpoint _outhit) (.normal _outhit) (.impactnormal _outhit) (.physmat _outhit) (.hitactor _outhit) (.hitcomponent _outhit) (.hitbonename _outhit) (.hititem _outhit) (.faceindex _outhit) (.tracestart _outhit) (.traceend _outhit)))))
        (elif (Variables|/Game/Blueprints/Blueprints/BP_Pawn_Palette.BP_Pawn_Palette_C|GetIsAbsorbing (Variables|Default|GetPawn_Palette))
          (CallFunction|AbsorbBrush "/Game/Assets/Characters/Palette/Paint/Texture_EraserAlpha.Texture_EraserAlpha" (Variables|Default|GetTargetBrushSize) (.UV (Class|GameplayStatics|FindCollisionUV (Collision|MakeHitResult (.bblockinghit _outhit) (.binitialoverlap _outhit) (.time _outhit) (.distance _outhit) (.location _outhit) (.impactpoint _outhit) (.normal _outhit) (.impactnormal _outhit) (.physmat _outhit) (.hitactor _outhit) (.hitcomponent _outhit) (.hitbonename _outhit) (.hititem _outhit) (.faceindex _outhit) (.tracestart _outhit) (.traceend _outhit))))))))))

(event EventBeginPlay
  (bind _paintablesurface (Variables|Default|GetPaintableSurface))
  (bind _rendertarget_size (Variables|Default|GetRenderTarget_Size))
  ;[1 1 1] Setup
  (Utilities|FlowControl|Sequence
    (:then_0
      ;;[1 1 1] Create Render Target / Brush Size
      (bind _returnvalue (Rendering|CreateRenderTarget2D _rendertarget_size _rendertarget_size "RTF_RGBA16f"))
      (bind _output_get (Variables|Default|SetRenderTarget _returnvalue))
      (Rendering|ClearRenderTarget2D _output_get)
      (Variables|Default|SetCurrentBrushSize (Variables|Default|GetTargetBrushSize)))
    (:then_1
      ;;[1 1 1] Canvas Material
      (bind _returnvalue_2 (Rendering|Material|CreateDynamicMaterialInstance (Variables|Default|GetCanvasMaterial) "None" "None" :!class /Script/Engine.KismetMaterialLibrary))
      (Rendering|Material|SetTextureParameterValue _returnvalue_2 "RenderTarget" (Variables|Default|GetRenderTarget))
      (Rendering|Material|SetTextureParameterValue _returnvalue_2 "ObjectMaterial_Albedo" (Variables|Default|GetObjectTexture_Albedo))
      (Rendering|Material|SetTextureParameterValue _returnvalue_2 "ObjectMaterial_ChannelPack" (Variables|Default|GetObjectTexture_ChannelPack))
      (Rendering|Material|SetTextureParameterValue _returnvalue_2 "ObjectMaterial_Normals" (Variables|Default|GetObjectTexture_Normals))
      (bind _output_get_2 (Variables|Default|SetCanvas _returnvalue_2))
      (Rendering|Material|SetMaterial (Variables|Default|GetPaintableSurface) 0 _output_get_2))
    (:then_2
      ;;[1 1 1] Eraser Material
      (bind _returnvalue_3 (Rendering|Material|CreateDynamicMaterialInstance "/Game/Assets/Characters/Palette/Paint/Mat_Eraser.Mat_Eraser" "None" "None" :!class /Script/Engine.KismetMaterialLibrary))
      (bind _output_get_3 (Variables|Default|SetEraserMaterial _returnvalue_3))
      (Rendering|Material|SetTextureParameterValue _output_get_3 "ObjectMaterial_Albedo" (Variables|Default|GetObjectTexture_Albedo))
      (Rendering|Material|SetScalarParameterValue _output_get_3 "Size" (Variables|Default|GetTargetBrushSize) :!class /Script/Engine.MaterialInstanceDynamic)
      (Rendering|Material|SetTextureParameterValue _output_get_3 "RenderTarget" (Variables|Default|GetRenderTarget)))
    (:then_3
      ;;[1 1 1] Set Render Custom Depth
      (Rendering|SetRenderCustomDepth _paintablesurface true)
      (Rendering|SetCustomDepthStencilValue _paintablesurface 1))))

(fn ConstructionScript)

(fn AbsorbBrush
  (params (BrushTexture :type Texture%202D%20Object%20Reference) (BrushSize :type Float%20%28single-precision%29) (DrawLocation :type Vector%202D%20Structure))
  (bind _targetbrushsize (Variables|Default|GetTargetBrushSize))
  (Utilities|FlowControl|Sequence
    (:then_0
      (Rendering|Material|SetTextureParameterValue (Variables|Default|GetEraserMaterial) "BrushMask" BrushTexture))
    (:then_1
      (bind (_canvas _size _context) (Rendering|BeginDrawCanvastoRenderTarget (Variables|Default|GetRenderTarget)))
      (Canvas|DrawMaterial :self _canvas :RenderMaterial (Variables|Default|GetEraserMaterial) :ScreenPosition (- (* _size DrawLocation) (/ _targetbrushsize 2.0)) :ScreenSize (Math|Vector2D|MakeVector2D _targetbrushsize _targetbrushsize) :CoordinateSize "(X=1.000000,Y=1.000000)" :Rotation (Math|Random|RandomFloatinRange 0.0 3.6e+02) :PivotPoint "(X=0.500000,Y=0.500000)")
      (Rendering|EndDrawCanvastoRenderTarget _context))))

(fn DrawBrushNew
  (params (BrushSize :type Float%20%28single-precision%29) (DrawLocation :type Vector%202D%20Structure))
  (bind _pawn_palette (Variables|Default|GetPawn_Palette))
  (bind _targetbrushsize (Variables|Default|GetTargetBrushSize))
  (Utilities|FlowControl|Sequence
    (:then_0
      (Variables|Default|SetBrushMaterial (Utilities|Array|Get(acopy) (Variables|/Game/Blueprints/Blueprints/BP_Pawn_Palette.BP_Pawn_Palette_C|GetPaint_Brushes _pawn_palette) (Variables|/Game/Blueprints/Blueprints/BP_Pawn_Palette.BP_Pawn_Palette_C|GetCurrentPaintColor_Index _pawn_palette))))
    (:then_1
      (bind (_canvas _size _context) (Rendering|BeginDrawCanvastoRenderTarget (Variables|Default|GetRenderTarget)))
      (Canvas|DrawMaterial :self _canvas :RenderMaterial (Variables|Default|GetBrushMaterial) :ScreenPosition (- (* _size DrawLocation) (/ _targetbrushsize 2.0)) :ScreenSize (Math|Vector2D|MakeVector2D _targetbrushsize _targetbrushsize) :CoordinateSize "(X=1.000000,Y=1.000000)" :Rotation (Math|Random|RandomFloatinRange 0.0 3.6e+02) :PivotPoint "(X=0.500000,Y=0.500000)")
      (Rendering|EndDrawCanvastoRenderTarget _context))))

(fn DrawBrushShade
  (params (BrushSize :type Float%20%28single-precision%29) (DrawLocation :type Vector%202D%20Structure))
  (bind _shade_targetbrushsize (Variables|Default|GetShade_TargetBrushSize))
  (bind (_canvas _size _context) (Rendering|BeginDrawCanvastoRenderTarget (Variables|Default|GetRenderTarget)))
  (Canvas|DrawMaterial :self _canvas :RenderMaterial (Variables|Default|GetShadeBrushMaterial) :ScreenPosition (- (* _size DrawLocation) (/ _shade_targetbrushsize 2.0)) :ScreenSize (Math|Vector2D|MakeVector2D _shade_targetbrushsize _shade_targetbrushsize) :CoordinateSize "(X=1.000000,Y=1.000000)" :Rotation (Math|Random|RandomFloatinRange 0.0 3.6e+02) :PivotPoint "(X=0.500000,Y=0.500000)")
  (Rendering|EndDrawCanvastoRenderTarget _context))

(fn ShadePaintTrace
  ;[1 1 1] Line trace for each shade paint orb
  (bind _outactors (Actor|GetAllActorsOfClass "/Game/Blueprints/Blueprints/BP_Shade_PaintObject.BP_Shade_PaintObject_C"))
  (for _array_element _outactors
    (if (not (Variables|/Game/Blueprints/Blueprints/BP_Shade_PaintObject.BP_Shade_PaintObject_C|GetHasSplatted _array_element))
      (Utilities|FlowControl|Sequence
        (:then_0
          (bind (_outhit _returnvalue) (Collision|LineTraceForObjects (Transformation|GetWorldLocation (Variables|/Game/Blueprints/Blueprints/BP_Shade_PaintObject.BP_Shade_PaintObject_C|GetPaintArrow _array_element)) (+ (Transformation|GetWorldLocation (Variables|/Game/Blueprints/Blueprints/BP_Shade_PaintObject.BP_Shade_PaintObject_C|GetPaintArrow _array_element)) (* (Math|Vector|GetForwardVector (Transformation|GetWorldRotation (Variables|/Game/Blueprints/Blueprints/BP_Shade_PaintObject.BP_Shade_PaintObject_C|GetPaintArrow _array_element))) (Variables|Default|GetLineTraceDistance))) (Utilities|Array|MakeArray "ObjectTypeQuery1") true 0 "ForDuration" false))
          (if (== (.hitactor _outhit) self)
            (if _returnvalue
              _
              (else
                _))
            (CallFunction|DrawBrushShade 0.0 (.UV (Class|GameplayStatics|FindCollisionUV (Collision|MakeHitResult (.bblockinghit _outhit) (.binitialoverlap _outhit) (.time _outhit) (.distance _outhit) (.location _outhit) (.impactpoint _outhit) (.normal _outhit) (.impactnormal _outhit) (.physmat _outhit) (.hitactor _outhit) (.hitcomponent _outhit) (.hitbonename _outhit) (.hititem _outhit) (.faceindex _outhit) (.tracestart _outhit) (.traceend _outhit)))))))
        (:then_1
          (Variables|/Game/Blueprints/Blueprints/BP_Shade_PaintObject.BP_Shade_PaintObject_C|SetHasSplatted _array_element true))))))