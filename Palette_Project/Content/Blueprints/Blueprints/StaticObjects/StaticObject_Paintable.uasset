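; Paintable static object whose surface receives paint from the PawnPalette's paint arrow.
; Construction creates dynamic canvas and splat materials; BeginPlay clears a new render target and feeds it to the canvas as its alpha.
; Each tick, a complex line trace along the arrow converts any WorldStatic hit to a UV position for the splat.
; While painting, the splat is drawn into the render target, without checking which object was hit.
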(event EventBeginPlay
  ;[1 1 1] Render Target Setup
  (bind _returnvalue (Rendering|CreateRenderTarget2D 2048 2048 "RTF_RGBA16f"))
  (Variables|Default|SetRenderTarget _returnvalue)
  (Rendering|ClearRenderTarget2D (Variables|Default|GetRenderTarget))
  (Rendering|Material|SetTextureParameterValue (Variables|Default|GetCanvas) "Alpha" (Variables|Default|GetRenderTarget)))

(event Collision|EventActorBeginOverlap
  (params (OtherActor :type Actor%20Object%20Reference)))

(event EventTick
  (params (DeltaSeconds :type Float%20%28single-precision%29))
  (bind _pawn_palette (Variables|Default|GetPawn_Palette))
  (bind _paintarrow (Variables|/Game/Blueprints/Blueprints/Pawn_Palette.Pawn_Palette_C|GetPaintArrow _pawn_palette))
  (bind _returnvalue (Transformation|GetWorldLocation _paintarrow))
  ;[1 1 1] Find Paint Location / Render Target
  (bind (_outhit _returnvalue_2) (Collision|LineTraceForObjects _returnvalue (+ _returnvalue (* (Math|Vector|GetForwardVector (Transformation|GetWorldRotation _paintarrow)) (Variables|Default|GetLineTraceDistance))) (Utilities|Array|MakeArray "ObjectTypeQuery1") true 0 "ForOneFrame" false))
  (if _returnvalue_2
    (Rendering|Material|SetVectorParameterValue (Variables|Default|GetSplat) "Position" (Utilities|Struct|MakeLinearColor (.x (.UV (Class|GameplayStatics|FindCollisionUV _outhit))) (.y (.UV (Class|GameplayStatics|FindCollisionUV _outhit))) 0.0 1.0) :!class /Script/Engine.MaterialInstanceDynamic)
    (if (Variables|/Game/Blueprints/Blueprints/Pawn_Palette.Pawn_Palette_C|GetIsPainting (Variables|Default|GetPawn_Palette))
      (Rendering|DrawMaterialtoRenderTarget (Variables|Default|GetRenderTarget) (Variables|Default|GetSplat)))))

(fn ConstructionScript
  (bind _returnvalue (Rendering|Material|CreateDynamicMaterialInstance "/Game/Assets/Characters/Palette/Paint/Mat_Canvas.Mat_Canvas" "None" "None" :!class /Script/Engine.KismetMaterialLibrary))
  (bind _output_get (Variables|Default|SetCanvas _returnvalue))
  (Rendering|Material|SetMaterial (Variables|Default|GetPaintableSurface) 0 _output_get)
  (bind _returnvalue_2 (Rendering|Material|CreateDynamicMaterialInstance "/Game/Assets/Characters/Palette/Paint/Mat_Splat.Mat_Splat" "None" "None" :!class /Script/Engine.KismetMaterialLibrary))
  (bind _output_get_2 (Variables|Default|SetSplat _returnvalue_2))
  (Rendering|Material|SetScalarParameterValue _output_get_2 "Size" 0.05 :!class /Script/Engine.MaterialInstanceDynamic)
  (Rendering|Material|SetTextureParameterValue _output_get_2 "BrushMask" "/Game/Assets/Characters/Palette/Paint/Texture_PaintAlpha_V1.Texture_PaintAlpha_V1"))