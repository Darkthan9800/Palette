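; Palette pawn that chases the mouse cursor through the world, painting and absorbing colored paint objects until frozen, with Interact unfreezing it.
; Tick interpolates it toward the cursor trace hit, drifting on momentum from its last known position when the trace misses or movement is disabled.
; Sphere overlaps at the cursor recolor existing paint or spawn new paint, draining the easel's blue, red or yellow supply; absorbing destroys paint to refill it.
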(event Custom|Freeze
  ;[1 1 1] Shade Action Freeze
  (Variables|Default|SetIsFrozen true)
  (Variables|Default|SetCanPaint false)
  (Variables|Default|SetCanMove false))

(event Custom|Unfreeze
  ;[1 1 1] Shade Action Freeze
  (Variables|Default|SetIsFrozen false)
  (Variables|Default|SetCanPaint true)
  (Variables|Default|SetCanMove true))

(event EventBeginPlay
  (bind _easelreference (Variables|Default|GetEaselReference))
  (bind _palette_skeletal (Variables|Default|GetPalette_Skeletal))
  (bind _camera1 (Variables|Default|GetCamera1))
  (bind _cursortoworld (Variables|Default|GetCursorToWorld))
  (bind _returnvalue (Transformation|GetActorLocation _easelreference))
  ;[1 1 1] Event Begin Play
  (bind _asbp_palette_gamemode (Utilities|Casting|CastToBP_Palette_Gamemode (Game|GetGameMode)))
  (bind _output_get (Variables|Default|SetPalette_Gamemode _asbp_palette_gamemode))
  (bind _returnvalue_2 (Class|GameModeBase|GetNumPlayers _output_get))
  (if (== _returnvalue_2 1)
    (Components|Activation|Deactivate _camera1)
    (Rendering|SetVisibility _cursortoworld false false)
    (else
      (Components|Activation|Activate _camera1 false)
      (Rendering|SetVisibility _cursortoworld true false)))
  ;;[0 1 0.06035] Beginning Location
  (Transformation|SetActorLocation (Math|Vector|MakeVector (.x _returnvalue) (+ (.y _returnvalue) 1e+02) (.z _returnvalue)) false false)
  (Input|EnableInput (Game|GetPlayerController 0))
  (Rendering|SetRenderCustomDepth _palette_skeletal true)
  (Rendering|SetCustomDepthStencilValue _palette_skeletal 0))

(event Collision|EventActorBeginOverlap
  (params (OtherActor :type Actor%20Object%20Reference)))

(event EventTick
  (params (DeltaSeconds :type Float%20%28single-precision%29))
  (bind _returnvalue (Transformation|GetActorLocation))
  (bind _returnvalue_2 (Game|GetPlayerController 0))
  (bind _currentpaintcolor_index (Variables|Default|GetCurrentPaintColor_Index))
  (bind _easelreference (Variables|Default|GetEaselReference))
  (bind _paintobject_recharge (Variables|Default|GetPaintObject_Recharge))
  (bind _paintobject_depletion (Variables|Default|GetPaintObject_Depletion))
  (bind _easelreference_2 (Variables|Default|GetEaselReference))
  (bind (_hitresult _returnvalue_3) (Game|Player|GetHitResultUnderCursorbyChannel _returnvalue_2 "TraceTypeQuery1" true))
  (bind (_bblockinghit _binitialoverlap _time _distance _location _impactpoint _normal _impactnormal) (Collision|BreakHitResult _hitresult))
  (bind _returnvalue_4 (Math|Vector|MakeVector (.x _location) (.y _location) (.z _location)))
  (bind _returnvalue_5 (Math|Vector|GetUnitDirection(Vector) _returnvalue _returnvalue_4))
  (bind _returnvalue_6 (Math|Conversions|RotationFromXVector _returnvalue_5))
  ;[1 1 1] Event Tick
  (Variables|Default|SetDeltaSeconds DeltaSeconds)
  (Utilities|FlowControl|Sequence
    (:then_0
      ;;[0 1 0.06268] Set Location and Rotation
      (if (and _returnvalue_3 (Variables|Default|GetCanMove))
        (bind _returnvalue_7 (CallFunction|GetMovementInterpolation (.x _location) (.y _location) (.z _location)))
        (bind _output_get (Variables|Default|SetLastKnownLocation _returnvalue_7))
        (Variables|Default|SetTargetRotation _returnvalue_6)
        (bind _output_get_2 (Variables|Default|SetLastKnownRotation (Class|KismetMathLibrary|RInterptoConstant (Transformation|GetActorRotation) _returnvalue_6 (Variables|Default|GetDeltaSeconds) 5e+02)))
        (Transformation|SetActorLocationAndRotation _output_get _output_get_2)
        (else
          (bind _targetlocation (CallFunction|LostLocationMomentum))
          (bind _returnvalue_8 (CallFunction|GetMovementInterpolation (.x _targetlocation) (.y _targetlocation) (.z _targetlocation)))
          (Transformation|SetActorLocationAndRotation _returnvalue_8 _output_get_2)))
      (Transformation|SetWorldLocationAndRotation (Variables|Default|GetCursorToWorld) _returnvalue_4 (Math|Rotator|MakeRotationfromAxes (Math|Vector|MakeVector (.x _impactnormal) (.y _impactnormal) (.z _impactnormal)) "0, 0, 0" "0, 0, 0") false false)
      ;;[0 0.03417 1] Painting
      (if (Math|Boolean|ANDBoolean (Variables|Default|GetIsPainting) (Variables|Default|GetCanPaint) (not (Variables|/Game/Blueprints/Blueprints/BP_Pawn_Easel.BP_Pawn_Easel_C|GetCurrentPaintEmpty (Variables|Default|GetEaselReference))))
        (bind (_outactors _returnvalue_9) (Collision|SphereOverlapActors (Transformation|GetWorldLocation (Variables|Default|GetCursorToWorld)) 75.0 (Utilities|Array|MakeArray "ObjectTypeQuery2") "/Game/Blueprints/Blueprints/BP_PaintObject.BP_PaintObject_C"))
        (Variables|Default|SetIsOverlappingPaintObject _returnvalue_9)
        (if (Variables|Default|GetIsOverlappingPaintObject)
          (for _array_element _outactors
            (bind _asbp_paint_object (Utilities|Casting|CastToBP_PaintObject _array_element))
            (Variables|/Game/Blueprints/Blueprints/BP_PaintObject.BP_PaintObject_C|SetPaintObject_Color _asbp_paint_object (Variables|Default|GetCurrentPaintColor_Index)))
          (else
            (Game|SpawnActorfromClass "/Game/Blueprints/Blueprints/BP_PaintObject.BP_PaintObject_C" (Math|Transform|MakeTransform _returnvalue_4) "AlwaysSpawn" 0 _currentpaintcolor_index 0)
            (switch int _currentpaintcolor_index
              (:0
                (Variables|/Game/Blueprints/Blueprints/BP_Pawn_Easel.BP_Pawn_Easel_C|SetPaintAmount_Blue _easelreference_2 (- (Variables|/Game/Blueprints/Blueprints/BP_Pawn_Easel.BP_Pawn_Easel_C|GetPaintAmount_Blue _easelreference_2) _paintobject_depletion)))
              (:1
                (Variables|/Game/Blueprints/Blueprints/BP_Pawn_Easel.BP_Pawn_Easel_C|SetPaintAmount_Red _easelreference_2 (- (Variables|/Game/Blueprints/Blueprints/BP_Pawn_Easel.BP_Pawn_Easel_C|GetPaintAmount_Red _easelreference_2) _paintobject_depletion)))
              (:2
                (Variables|/Game/Blueprints/Blueprints/BP_Pawn_Easel.BP_Pawn_Easel_C|SetPaintAmount_Yellow _easelreference_2 (- (Variables|/Game/Blueprints/Blueprints/BP_Pawn_Easel.BP_Pawn_Easel_C|GetPaintAmount_Yellow _easelreference_2) _paintobject_depletion))))))
        (else
          ;;[0 0.03342 1] Absorbing
          (if (Variables|Default|GetIsAbsorbing)
            (bind (_outactors_2 _returnvalue_10) (Collision|SphereOverlapActors (Transformation|GetWorldLocation (Variables|Default|GetCursorToWorld)) 75.0 (Utilities|Array|MakeArray "ObjectTypeQuery2") "/Game/Blueprints/Blueprints/BP_PaintObject.BP_PaintObject_C"))
            (bind _array_element_2 (Utilities|Array|ForEachLoopwithBreak _outactors_2)
              (:LoopBody
                (bind _asbp_paint_object_2 (Utilities|Casting|CastToBP_PaintObject _array_element_2))
                (Variables|Default|SetPaintObjectReference _asbp_paint_object_2)
                (if _returnvalue_10
                  (switch int (Variables|/Game/Blueprints/Blueprints/BP_PaintObject.BP_PaintObject_C|GetPaintObject_Color (Variables|Default|GetPaintObjectReference))
                    (:0
                      (Variables|/Game/Blueprints/Blueprints/BP_Pawn_Easel.BP_Pawn_Easel_C|SetPaintAmount_Blue _easelreference (+ (Variables|/Game/Blueprints/Blueprints/BP_Pawn_Easel.BP_Pawn_Easel_C|GetPaintAmount_Blue _easelreference) _paintobject_recharge)))
                    (:1
                      (Variables|/Game/Blueprints/Blueprints/BP_Pawn_Easel.BP_Pawn_Easel_C|SetPaintAmount_Red _easelreference (+ (Variables|/Game/Blueprints/Blueprints/BP_Pawn_Easel.BP_Pawn_Easel_C|GetPaintAmount_Red _easelreference) _paintobject_recharge)))
                    (:2
                      (Variables|/Game/Blueprints/Blueprints/BP_Pawn_Easel.BP_Pawn_Easel_C|SetPaintAmount_Yellow _easelreference (+ (Variables|/Game/Blueprints/Blueprints/BP_Pawn_Easel.BP_Pawn_Easel_C|GetPaintAmount_Yellow _easelreference) _paintobject_recharge))))
                  (Actor|DestroyActor _array_element_2))))))))))

(event EventInteract
  (CallFunction|Unfreeze))

(fn ConstructionScript)

(fn LostLocationMomentum
  (bind _returnvalue (Transformation|GetActorLocation))
  (bind _cursortoworld (Variables|Default|GetCursorToWorld))
  (bind _returnvalue_2 (Transformation|GetWorldLocation _cursortoworld))
  (Variables|Default|SetMomentumDistance (/ (Math|Float|Sqrt (+ (Math|Float|Square (- (.x _returnvalue) (.x _returnvalue_2))) (Math|Float|Square (- (.y _returnvalue) (.y _returnvalue_2))) (Math|Float|Square (- (.z _returnvalue) (.z _returnvalue_2))))) 8.0))
  (return (+ (Variables|Default|GetLastKnownLocation) (* (Math|Vector|GetForwardVector (Variables|Default|GetTargetRotation)) (Variables|Default|GetMomentumDistance)))))

(fn GetMovementInterpolation
  (params (Target_X :type Float%20%28single-precision%29) (Target_Y :type Float%20%28single-precision%29) (Target_Z :type Float%20%28single-precision%29))
  (bind _returnvalue (Transformation|GetActorLocation))
  (bind _deltaseconds (Variables|Default|GetDeltaSeconds))
  (return (Math|Vector|MakeVector (Math|Interpolation|FInterpTo (.x _returnvalue) Target_X _deltaseconds 6.0) (Math|Interpolation|FInterpTo (.y _returnvalue) Target_Y _deltaseconds 6.0) (Math|Interpolation|FInterpTo (.z _returnvalue) Target_Z _deltaseconds 6.0))))